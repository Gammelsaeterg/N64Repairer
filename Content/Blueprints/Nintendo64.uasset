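; Nintendo 64 console actor whose power switch turns the console on and off and controls video playback on a linked TV.
; BeginPlay creates a dynamic material instance on the console mesh, and each switch event flips Power and a scalar parameter on that material.
; StartTV and PauseTV play or pause CurrentTv's media player, each through its own FlipFlop, so they act only on alternate calls.
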(event `self.ReceiveBeginPlay`
  (bind _returnvalue (`PrimitiveComponent.CreateDynamicMaterialInstance` (`self.NintendoMesh`) 0 "/Game/Materials/N64Mat.N64Mat" "None"))
  (set `self.MatInst` _returnvalue)
  (`PrimitiveComponent.SetMaterial` (`self.NintendoMesh`) 0 _returnvalue))

(event `NintendoPowerSwitch`
  (`/Engine/EditorBlueprintResources/StandardMacros.FlipFlop`
    (:`A`
      (`self.StartTV`)
      (set `self.Power` true)
      (`MaterialInstanceDynamic.SetScalarParameterValue` (`self.MatInst`) "Param" 100.0))
    (:`B`
      (`self.PauseTV`)
      (set `self.Power` false)
      (`MaterialInstanceDynamic.SetScalarParameterValue` (`self.MatInst`) "Param" 0.0))))

(fn `PauseTV`
  (`/Engine/EditorBlueprintResources/StandardMacros.IsValid` (`self.CurrentTv`)
    (:`Is Valid`
      (`/Engine/EditorBlueprintResources/StandardMacros.FlipFlop`
        (:`A`
          (`MediaPlayer.Pause` (`/Game/Blueprints/TVScreen_Blueprint.MediaPlayer1` (`self.CurrentTv`))))))))

(fn `StartTV`
  (`/Engine/EditorBlueprintResources/StandardMacros.IsValid` (`self.CurrentTv`)
    (:`Is Valid`
      (`/Engine/EditorBlueprintResources/StandardMacros.FlipFlop`
        (:`A`
          (`MediaPlayer.Play` (`/Game/Blueprints/TVScreen_Blueprint.MediaPlayer1` (`self.CurrentTv`))))))))

(fn `UserConstructionScript`)